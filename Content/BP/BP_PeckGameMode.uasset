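; BP_PeckGameMode is a game mode that runs a minutes-and-seconds countdown and keeps a score.
; Tick passes through a one-second Delay to decrement Seconds, rolling over into Minutes, and quits the game when both reach zero.
; Score resets to zero on BeginPlay and rises by one on each AddScore event.
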(event Custom|AddScore
  (Variables|Default|SetScore (+ (Variables|Default|GetScore) 1)))

(event EventTick
  (params (DeltaSeconds :type Float%20%28single-precision%29))
  (Utilities|FlowControl|Delay 1.0)
  (Variables|Default|SetSeconds (- (Variables|Default|GetSeconds) 1))
  (if (< (Variables|Default|GetSeconds) 0)
    (Variables|Default|SetMinutes (- (Variables|Default|GetMinutes) 1))
    (Variables|Default|SetSeconds 59))
  (if (== (Variables|Default|GetSeconds) 0)
    (if (== (Variables|Default|GetMinutes) 0)
      (Game|QuitGame 0 "Quit"))))

(event EventBeginPlay
  (Variables|Default|SetScore 0))

(fn ConstructionScript)